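; Player Blueprint for a train test that rides along the spline of the first BP_TrackGenerator found in the level.
; Accelerate and Deccelerate presses latch forward or backward movement, which Tick turns into timeline play or reverse, wrapping at either end.
; The timeline's alpha maps to distance along the spline, setting player pawn 0's world location and rotation.
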(event EventTick
  (params (DeltaSeconds :type Float%20%28single-precision%29))
  (bind _track (Variables|Default|GetTrack))
  (bind _spline (Variables|/Game/TrainTest/BP_TrackGenerator.BP_TrackGenerator_C|GetSpline _track))
  (if (Variables|Default|GetMoveForward)
    (if (== (Variables|Default|GetAlpha) 1.0)
      (bind _alpha (Timeline|Timeline_0 PlayFromStart)
        (:Update
          (bind _output_get (Variables|Default|SetAlpha _alpha))
          (Transformation|SetActorLocationAndRotation (Game|Player|GetPlayerPawn 0) (Spline|GetLocationatDistanceAlongSpline _spline (Math|Float|Lerp 0.0 (Spline|GetSplineLength _spline) _output_get) "World") (Spline|GetRotationatDistanceAlongSpline _spline (Math|Float|Lerp 0.0 (Spline|GetSplineLength _spline) _output_get) "World"))))
      (else
        (Timeline|Timeline_0 Play)))
    (elif (Variables|Default|GetMoveBackward)
      (if (== (Variables|Default|GetAlpha) 0.0)
        (Timeline|Timeline_0 ReverseFromEnd)
        (else
          (Timeline|Timeline_0 Reverse)))
      (else
        (Timeline|Timeline_0 Stop)))))

(event EventBeginPlay
  (bind _outactors (Actor|GetAllActorsOfClass "/Game/TrainTest/BP_TrackGenerator.BP_TrackGenerator_C"))
  (Variables|Default|SetTrack (Utilities|Array|Get(acopy) _outactors))
  (Components|Timeline|SetPlayRate (Variables|Default|GetTimeline_0) 0.2))

(event Input|ActionEvents|InputActionAccelerate
  (params (Key :type Key%20Structure))
  (:Pressed
    (Variables|Default|SetMoveBackward false)
    (Variables|Default|SetMoveForward true)))

(event Input|ActionEvents|InputActionDeccelerate
  (params (Key :type Key%20Structure))
  (:Pressed
    (Variables|Default|SetMoveForward false)
    (Variables|Default|SetMoveBackward true)))

(fn ConstructionScript)