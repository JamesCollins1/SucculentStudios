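; Track generator actor that builds a track along an editable spline in the construction script.
; It resizes the TrackData array to match the spline point count, then CreateTrack adds one spline mesh per point using TrackMesh.
; Each segment takes local locations and tangents from its point and the next, with a modulo wrap that closes the loop.
; TrackData entries are not read when building segments.
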(event EventBeginPlay)

(event Collision|EventActorBeginOverlap
  (params (OtherActor :type Actor%20Object%20Reference)))

(event EventTick
  (params (DeltaSeconds :type Float%20%28single-precision%29)))

(fn ConstructionScript
  (bind _trackdata (Variables|Default|GetTrackData))
  (bind _trackdata_2 (Variables|Default|GetTrackData))
  (Utilities|FlowControl|Sequence
    (:then_0
      (Variables|Default|SetSplinePoints (Spline|GetNumberOfSplinePoints (Variables|Default|GetSpline))))
    (:then_1
      (Math|Integer|CompareInt (Utilities|Array|Length _trackdata_2) (Variables|Default|GetSplinePoints) :!label _label
        (:>
          (Utilities|Array|RemoveIndex _trackdata (Utilities|Array|LastIndex _trackdata))
          (goto _label))
        (:<
          (Utilities|Array|Add :TargetArray _trackdata_2)
          (goto _label))))
    (:then_2
      (for _index (range 0 (- (Variables|Default|GetSplinePoints) 1))
        (CallFunction|CreateTrack _index (Variables|Default|GetTrackMesh))))))

(fn CreateTrack
  (params (CurrentLoopIndex :type Integer) (Mesh :type Static%20Mesh%20Object%20Reference))
  (LocalVariables|SetLocalCurrentLoopIndex CurrentLoopIndex)
  (LocalVariables|SetLocalNextLoopIndex (Math|Integer|%(Integer) (+ CurrentLoopIndex 1) (Variables|Default|GetSplinePoints)))
  (LocalVariables|SetLocalTrackElementMesh Mesh)
  (Utilities|FlowControl|Sequence
    (:then_0
      (LocalVariables|SetLocalStartTangent (.Tangent (Spline|GetLocationandTangentatSplinePoint (Variables|Default|GetSpline) (LocalVariables|GetLocalCurrentLoopIndex) "Local")))
      (LocalVariables|SetLocalStartLocation (.Location (Spline|GetLocationandTangentatSplinePoint (Variables|Default|GetSpline) (LocalVariables|GetLocalCurrentLoopIndex) "Local")))
      (LocalVariables|SetLocalEndTangent (.Tangent (Spline|GetLocationandTangentatSplinePoint (Variables|Default|GetSpline) (LocalVariables|GetLocalNextLoopIndex) "Local")))
      (LocalVariables|SetLocalEndLocation (.Location (Spline|GetLocationandTangentatSplinePoint (Variables|Default|GetSpline) (LocalVariables|GetLocalNextLoopIndex) "Local"))))
    (:then_1
      (bind _returnvalue (AddComponent|AddSplineMeshComponent false))
      (bind _output_get (LocalVariables|SetCurrentSplineMesh _returnvalue))
      (Components|StaticMesh|SetStaticMesh _output_get (LocalVariables|GetLocalTrackElementMesh))
      (SplineMesh|SetStartandEnd (LocalVariables|GetCurrentSplineMesh) (LocalVariables|GetLocalStartLocation) (LocalVariables|GetLocalStartTangent) (LocalVariables|GetLocalEndLocation) (LocalVariables|GetLocalEndTangent) true :!class /Script/Engine.SplineMeshComponent))))